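; GrayChan sample actor that demonstrates KawaiiPhysics on an animated mesh, with optional movement and physics overrides.
; When Move is set, a timeline started on BeginPlay drives the GrayChan component's relative Y location.
; When OverridePhysicsSettings is set, BeginPlay and every Tick copy the actor's physics, dummy bone, teleport threshold, gravity, wind and collision variables into AnimBP_GrayChanKawaiiPhysics.
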(event EventBeginPlay
  (Utilities|FlowControl|Sequence
    (:then_0
      (if (Variables|Default|GetbMove)
        (bind _newtrack_0 (Timeline|Timeline_0 PlayFromStart)
          (:Update
            (Transformation|SetRelativeLocation (Variables|Default|GetGrayChan) (Math|Vector|MakeVector 0.0 (* _newtrack_0 9e+01) 0.0) false false)))))
    (:then_1
      (if (Variables|Default|GetbOverridePhysicsSettings)
        (bind _asanim_bp_gray_chan_kawaii_physics (Utilities|Casting|CastToAnimBP_GrayChanKawaiiPhysics (Components|SkeletalMesh|GetAnimInstance (Variables|Default|GetGrayChan))))
        (Utilities|FlowControl|Sequence
          (:then_0
            (Variables|/Game/KawaiiPhysicsSample/GrayChan/AnimBP_GrayChanKawaiiPhysics.AnimBP_GrayChanKawaiiPhysics_C|SetPhysicsSettings _asanim_bp_gray_chan_kawaii_physics (Variables|Default|GetPhysicsSettings))
            (Variables|/Game/KawaiiPhysicsSample/GrayChan/AnimBP_GrayChanKawaiiPhysics.AnimBP_GrayChanKawaiiPhysics_C|SetDummyBoneLength _asanim_bp_gray_chan_kawaii_physics (Variables|Default|GetDummyBoneLength))
            (Variables|/Game/KawaiiPhysicsSample/GrayChan/AnimBP_GrayChanKawaiiPhysics.AnimBP_GrayChanKawaiiPhysics_C|SetTeleport%20Distance%20Threshold _asanim_bp_gray_chan_kawaii_physics (Variables|Default|GetTeleport%20Distance%20Threshold))
            (Variables|/Game/KawaiiPhysicsSample/GrayChan/AnimBP_GrayChanKawaiiPhysics.AnimBP_GrayChanKawaiiPhysics_C|SetTeleport%20Roattion%20Threshold _asanim_bp_gray_chan_kawaii_physics (Variables|Default|GetTeleport%20Roattion%20Threshold)))
          (:then_1
            (Variables|/Game/KawaiiPhysicsSample/GrayChan/AnimBP_GrayChanKawaiiPhysics.AnimBP_GrayChanKawaiiPhysics_C|SetGravity _asanim_bp_gray_chan_kawaii_physics (Variables|Default|GetGravity))
            (Variables|/Game/KawaiiPhysicsSample/GrayChan/AnimBP_GrayChanKawaiiPhysics.AnimBP_GrayChanKawaiiPhysics_C|SetEnableWind _asanim_bp_gray_chan_kawaii_physics (Variables|Default|GetEnableWind))
            (Variables|/Game/KawaiiPhysicsSample/GrayChan/AnimBP_GrayChanKawaiiPhysics.AnimBP_GrayChanKawaiiPhysics_C|SetEnableCollision _asanim_bp_gray_chan_kawaii_physics (Variables|Default|GetEnableCollision))))))))

(event Collision|EventActorBeginOverlap
  (params (OtherActor :type Actor%20Object%20Reference)))

(event EventTick
  (params (DeltaSeconds :type Float%20%28single-precision%29))
  (if (Variables|Default|GetbOverridePhysicsSettings)
    (bind _asanim_bp_gray_chan_kawaii_physics (Utilities|Casting|CastToAnimBP_GrayChanKawaiiPhysics (Components|SkeletalMesh|GetAnimInstance (Variables|Default|GetGrayChan))))
    (Utilities|FlowControl|Sequence
      (:then_0
        (Variables|/Game/KawaiiPhysicsSample/GrayChan/AnimBP_GrayChanKawaiiPhysics.AnimBP_GrayChanKawaiiPhysics_C|SetPhysicsSettings _asanim_bp_gray_chan_kawaii_physics (Variables|Default|GetPhysicsSettings))
        (Variables|/Game/KawaiiPhysicsSample/GrayChan/AnimBP_GrayChanKawaiiPhysics.AnimBP_GrayChanKawaiiPhysics_C|SetDummyBoneLength _asanim_bp_gray_chan_kawaii_physics (Variables|Default|GetDummyBoneLength))
        (Variables|/Game/KawaiiPhysicsSample/GrayChan/AnimBP_GrayChanKawaiiPhysics.AnimBP_GrayChanKawaiiPhysics_C|SetTeleport%20Distance%20Threshold _asanim_bp_gray_chan_kawaii_physics (Variables|Default|GetTeleport%20Distance%20Threshold))
        (Variables|/Game/KawaiiPhysicsSample/GrayChan/AnimBP_GrayChanKawaiiPhysics.AnimBP_GrayChanKawaiiPhysics_C|SetTeleport%20Roattion%20Threshold _asanim_bp_gray_chan_kawaii_physics (Variables|Default|GetTeleport%20Roattion%20Threshold)))
      (:then_1
        (Variables|/Game/KawaiiPhysicsSample/GrayChan/AnimBP_GrayChanKawaiiPhysics.AnimBP_GrayChanKawaiiPhysics_C|SetGravity _asanim_bp_gray_chan_kawaii_physics (Variables|Default|GetGravity))
        (Variables|/Game/KawaiiPhysicsSample/GrayChan/AnimBP_GrayChanKawaiiPhysics.AnimBP_GrayChanKawaiiPhysics_C|SetEnableWind _asanim_bp_gray_chan_kawaii_physics (Variables|Default|GetEnableWind))
        (Variables|/Game/KawaiiPhysicsSample/GrayChan/AnimBP_GrayChanKawaiiPhysics.AnimBP_GrayChanKawaiiPhysics_C|SetEnableCollision _asanim_bp_gray_chan_kawaii_physics (Variables|Default|GetEnableCollision))))))

(fn ConstructionScript)