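; GrayChan sample actor that demonstrates Kawaii Physics secondary bone motion and exposes its settings on the actor.
; When Move is set, a timeline started at BeginPlay drives the GrayChan component's relative Y location.
; When OverridePhysicsSettings is set, BeginPlay and every Tick copy the actor's physics, teleport threshold, gravity, wind and collision values into ABP_GC_KawaiiPhysics, so changes apply live.
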(event EventBeginPlay
  (Utilities|FlowControl|Sequence
    (:then_0
      (if (Variables|Default|GetbMove)
        (bind _newtrack_0 (Timeline|Timeline_0 PlayFromStart)
          (:Update
            (Transformation|SetRelativeLocation (Variables|Default|GetGrayChan) (Math|Vector|MakeVector 0.0 (* _newtrack_0 9e+01) 0.0) false false)))))
    (:then_1
      (if (Variables|Default|GetbOverridePhysicsSettings)
        (bind _asabp_gray_chan_kawaii_physics (Utilities|Casting|CastToABP_GC_KawaiiPhysics (Components|SkeletalMesh|GetAnimInstance (Variables|Default|GetGrayChan))))
        (bind _output_get (Variables|Default|SetABP%20KawaiiPhysics _asabp_gray_chan_kawaii_physics))
        (Utilities|FlowControl|Sequence
          (:then_0
            (Variables|/Game/KawaiiPhysicsSample/GrayChan/ABP_GC_KawaiiPhysics.ABP_GC_KawaiiPhysics_C|SetPhysicsSettings _output_get (Variables|Default|GetPhysicsSettings))
            (Variables|/Game/KawaiiPhysicsSample/GrayChan/ABP_GC_KawaiiPhysics.ABP_GC_KawaiiPhysics_C|SetDummyBoneLength _output_get (Variables|Default|GetDummyBoneLength))
            (Variables|/Game/KawaiiPhysicsSample/GrayChan/ABP_GC_KawaiiPhysics.ABP_GC_KawaiiPhysics_C|SetTeleport%20Distance%20Threshold _output_get (Variables|Default|GetTeleport%20Distance%20Threshold))
            (Variables|/Game/KawaiiPhysicsSample/GrayChan/ABP_GC_KawaiiPhysics.ABP_GC_KawaiiPhysics_C|SetTeleport%20Roattion%20Threshold _output_get (Variables|Default|GetTeleport%20Roattion%20Threshold)))
          (:then_1
            (Variables|/Game/KawaiiPhysicsSample/GrayChan/ABP_GC_KawaiiPhysics.ABP_GC_KawaiiPhysics_C|SetGravity _output_get (Variables|Default|GetGravity))
            (Variables|/Game/KawaiiPhysicsSample/GrayChan/ABP_GC_KawaiiPhysics.ABP_GC_KawaiiPhysics_C|SetEnableWind _output_get (Variables|Default|GetEnableWind))
            (Variables|/Game/KawaiiPhysicsSample/GrayChan/ABP_GC_KawaiiPhysics.ABP_GC_KawaiiPhysics_C|SetEnableCollision _output_get (Variables|Default|GetEnableCollision))))))))

(event Collision|EventActorBeginOverlap
  (params (OtherActor :type Actor%20Object%20Reference)))

(event EventTick
  (params (DeltaSeconds :type Float%20%28single-precision%29))
  (if (Variables|Default|GetbOverridePhysicsSettings)
    (bind _asabp_gray_chan_kawaii_physics (Utilities|Casting|CastToABP_GC_KawaiiPhysics (Components|SkeletalMesh|GetAnimInstance (Variables|Default|GetGrayChan))))
    (bind _output_get (Variables|Default|SetABP%20KawaiiPhysics _asabp_gray_chan_kawaii_physics))
    (Utilities|FlowControl|Sequence
      (:then_0
        (Variables|/Game/KawaiiPhysicsSample/GrayChan/ABP_GC_KawaiiPhysics.ABP_GC_KawaiiPhysics_C|SetPhysicsSettings _output_get (Variables|Default|GetPhysicsSettings))
        (Variables|/Game/KawaiiPhysicsSample/GrayChan/ABP_GC_KawaiiPhysics.ABP_GC_KawaiiPhysics_C|SetDummyBoneLength _output_get (Variables|Default|GetDummyBoneLength))
        (Variables|/Game/KawaiiPhysicsSample/GrayChan/ABP_GC_KawaiiPhysics.ABP_GC_KawaiiPhysics_C|SetTeleport%20Distance%20Threshold _output_get (Variables|Default|GetTeleport%20Distance%20Threshold))
        (Variables|/Game/KawaiiPhysicsSample/GrayChan/ABP_GC_KawaiiPhysics.ABP_GC_KawaiiPhysics_C|SetTeleport%20Roattion%20Threshold _output_get (Variables|Default|GetTeleport%20Roattion%20Threshold)))
      (:then_1
        (Variables|/Game/KawaiiPhysicsSample/GrayChan/ABP_GC_KawaiiPhysics.ABP_GC_KawaiiPhysics_C|SetGravity _output_get (Variables|Default|GetGravity))
        (Variables|/Game/KawaiiPhysicsSample/GrayChan/ABP_GC_KawaiiPhysics.ABP_GC_KawaiiPhysics_C|SetEnableWind _output_get (Variables|Default|GetEnableWind))
        (Variables|/Game/KawaiiPhysicsSample/GrayChan/ABP_GC_KawaiiPhysics.ABP_GC_KawaiiPhysics_C|SetEnableCollision _output_get (Variables|Default|GetEnableCollision))))))

(fn ConstructionScript)