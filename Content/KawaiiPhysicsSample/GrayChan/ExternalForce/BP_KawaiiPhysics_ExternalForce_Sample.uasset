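; Sample Blueprint external force for KawaiiPhysics that pushes simulated bones along a configurable direction.
; PreApply builds the force from direction, scale and the node's delta time.
; Apply ignores the bone index, shifting every ModifyBone by the force converted to component space and multiplied again by its length, so magnitude grows quadratically.
; It then writes the bone array back to the anim node.
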(event EventPreApply
  (params (Node :type Anim%20Node%20Kawaii%20Physics%20Structure%20%28by%20ref%29) (SkelComp :type Skeletal%20Mesh%20Component%20Object%20Reference))
  (Variables|Default|SetForce (* (Variables|Default|GetForce%20Dir) (Variables|Default|GetForceScale) (.DeltaTime (Utilities|Struct|BreakAnimNode_KawaiiPhysics Node)))))

(fn Apply
  (params (Node :type Anim%20Node%20Kawaii%20Physics%20Structure%20%28by%20ref%29) (ModifyBoneIndex :type Integer) (SkelComp :type Skeletal%20Mesh%20Component%20Object%20Reference) (BoneTransform :type Transform%20%28by%20ref%29))
  (bind _force (Variables|Default|GetForce))
  (Utilities|FlowControl|Sequence
    (:then_0
      (bind _output_get (LocalVariables|SetModify%20Bones (.ModifyBones (Utilities|Struct|BreakAnimNode_KawaiiPhysics Node))))
      (for _array_element _output_get
        (Utilities|Struct|SetmembersinKawaiiPhysicsModifyBone _array_element (+ (.Location (Utilities|Struct|BreakKawaiiPhysicsModifyBone _array_element)) (* (Math|Transform|InverseTransformDirection (Transformation|GetWorldTransform SkelComp) _force) (Math|Vector|VectorLength _force))))))
    (:then_1
      (Utilities|Struct|SetmembersinAnimNode_KawaiiPhysics Node (LocalVariables|GetModify%20Bones))
      (return))))