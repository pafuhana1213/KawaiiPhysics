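; BP_Chain is a KawaiiPhysics sample actor that demonstrates bone physics on a chain mesh.
; When Move is set, a timeline started on BeginPlay drives the SChain component's relative Y location.
; When OverridePhysicsSettings is set, BeginPlay and every Tick copy the actor's physics, dummy bone, teleport threshold, gravity and wind values into the chain's AnimBP_ChainKawaiiPhysics instance.
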(event EventBeginPlay
  (Utilities|FlowControl|Sequence
    (:then_0
      (if (Variables|Default|GetbMove)
        (bind _newtrack_0 (Timeline|Timeline_0 PlayFromStart)
          (:Update
            (Transformation|SetRelativeLocation (Variables|Default|GetS_Chain) (Math|Vector|MakeVector 0.0 (* _newtrack_0 9e+01) 0.0) false false)))))
    (:then_1
      (if (Variables|Default|GetbOverridePhysicsSettings)
        (bind _asanim_bp_chain_kawaii_physics (Utilities|Casting|CastToAnimBP_ChainKawaiiPhysics (Components|SkeletalMesh|GetAnimInstance (Variables|Default|GetS_Chain))))
        (Utilities|FlowControl|Sequence
          (:then_0
            (Variables|/Game/KawaiiPhysicsSample/Chain/AnimBP_ChainKawaiiPhysics.AnimBP_ChainKawaiiPhysics_C|SetPhysicsSettings _asanim_bp_chain_kawaii_physics (Variables|Default|GetPhysicsSettings))
            (Variables|/Game/KawaiiPhysicsSample/Chain/AnimBP_ChainKawaiiPhysics.AnimBP_ChainKawaiiPhysics_C|SetDummyBoneLength _asanim_bp_chain_kawaii_physics (Variables|Default|GetDummyBoneLength))
            (Variables|/Game/KawaiiPhysicsSample/Chain/AnimBP_ChainKawaiiPhysics.AnimBP_ChainKawaiiPhysics_C|SetTeleport%20Distance%20Threshold _asanim_bp_chain_kawaii_physics (Variables|Default|GetTeleport%20Distance%20Threshold))
            (Variables|/Game/KawaiiPhysicsSample/Chain/AnimBP_ChainKawaiiPhysics.AnimBP_ChainKawaiiPhysics_C|SetTeleport%20Roattion%20Threshold _asanim_bp_chain_kawaii_physics (Variables|Default|GetTeleport%20Roattion%20Threshold)))
          (:then_1
            (Variables|/Game/KawaiiPhysicsSample/Chain/AnimBP_ChainKawaiiPhysics.AnimBP_ChainKawaiiPhysics_C|SetGravity _asanim_bp_chain_kawaii_physics (Variables|Default|GetGravity))
            (Variables|/Game/KawaiiPhysicsSample/Chain/AnimBP_ChainKawaiiPhysics.AnimBP_ChainKawaiiPhysics_C|SetWind _asanim_bp_chain_kawaii_physics (Variables|Default|GetWind))))))))

(event EventTick
  (params (DeltaSeconds :type Float%20%28single-precision%29))
  (if (Variables|Default|GetbOverridePhysicsSettings)
    (bind _asanim_bp_chain_kawaii_physics (Utilities|Casting|CastToAnimBP_ChainKawaiiPhysics (Components|SkeletalMesh|GetAnimInstance (Variables|Default|GetS_Chain))))
    (Utilities|FlowControl|Sequence
      (:then_0
        (Variables|/Game/KawaiiPhysicsSample/Chain/AnimBP_ChainKawaiiPhysics.AnimBP_ChainKawaiiPhysics_C|SetPhysicsSettings _asanim_bp_chain_kawaii_physics (Variables|Default|GetPhysicsSettings))
        (Variables|/Game/KawaiiPhysicsSample/Chain/AnimBP_ChainKawaiiPhysics.AnimBP_ChainKawaiiPhysics_C|SetDummyBoneLength _asanim_bp_chain_kawaii_physics (Variables|Default|GetDummyBoneLength))
        (Variables|/Game/KawaiiPhysicsSample/Chain/AnimBP_ChainKawaiiPhysics.AnimBP_ChainKawaiiPhysics_C|SetTeleport%20Distance%20Threshold _asanim_bp_chain_kawaii_physics (Variables|Default|GetTeleport%20Distance%20Threshold))
        (Variables|/Game/KawaiiPhysicsSample/Chain/AnimBP_ChainKawaiiPhysics.AnimBP_ChainKawaiiPhysics_C|SetTeleport%20Roattion%20Threshold _asanim_bp_chain_kawaii_physics (Variables|Default|GetTeleport%20Roattion%20Threshold)))
      (:then_1
        (Variables|/Game/KawaiiPhysicsSample/Chain/AnimBP_ChainKawaiiPhysics.AnimBP_ChainKawaiiPhysics_C|SetGravity _asanim_bp_chain_kawaii_physics (Variables|Default|GetGravity))
        (Variables|/Game/KawaiiPhysicsSample/Chain/AnimBP_ChainKawaiiPhysics.AnimBP_ChainKawaiiPhysics_C|SetWind _asanim_bp_chain_kawaii_physics (Variables|Default|GetWind))))))

(fn ConstructionScript)