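; Stage actor for the KawaiiPhysics sample that labels a demo stage with text, built entirely in the construction script.
; The main label is formatted from category index, stage index and main text.
; SetupTextRenderSub adds one text render component per entry of two sub-text arrays, spreading them evenly along Y over a fixed span under each array's root.
; Each non-empty row's root is then shifted by its offset.
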(event EventBeginPlay)

(event Collision|EventActorBeginOverlap
  (params (OtherActor :type Actor%20Object%20Reference)))

(event EventTick
  (params (DeltaSeconds :type Float%20%28single-precision%29)))

(fn ConstructionScript
  (Rendering|Components|TextRender|SetText (Variables|Default|GetTextRender_Main) (Utilities|Text|FormatText "{Category}-{Stage} {Text}" (Variables|Default|GetCategoryIndex) (Variables|Default|GetStageIndex) (Variables|Default|GetText_Main)))
  (CallFunction|SetupTextRenderSub (Variables|Default|GetText_Sub_0) (Variables|Default|GetRoot_TextRenderSub_0) (Variables|Default|GetOffset_0))
  (CallFunction|SetupTextRenderSub (Variables|Default|GetText_Sub_1) (Variables|Default|GetRoot_TextRenderSub_1) (Variables|Default|GetOffset_1)))

(fn SetupTextRenderSub
  (params (Texts :type Array%20of%20Texts) (Parent :type Scene%20Component%20Object%20Reference) (Offset :type Vector))
  (if (Utilities|Array|IsNotEmpty Texts)
    (Utilities|FlowControl|Sequence
      (:then_0
        ;[1 1 1] Add Text Render
        (LocalVariables|SetDistance (Math|Conversions|ToFloat(Integer) (/ 1000 (+ (Utilities|Array|Length Texts) 1))))
        (for (_array_element _array_index) Texts
          (Utilities|FlowControl|Sequence
            (:then_0
              (bind _returnvalue (AddComponent|AddTextRenderComponent false))
              (LocalVariables|SetAdded%20Text%20Render%20Comp _returnvalue)
              (Transformation|AttachComponentToComponent (LocalVariables|GetAdded%20Text%20Render%20Comp) Parent "None" "SnapToTarget" "SnapToTarget" "KeepRelative" true)
              (Transformation|SetRelativeLocationAndRotation (LocalVariables|GetAdded%20Text%20Render%20Comp) (Math|Vector|MakeVector 0.0 (* (+ _array_index 1) (LocalVariables|GetDistance)) 0.0) "0.000000,180.000000,0.000000" false false))
            (:then_1
              (Rendering|Components|TextRender|SetText (LocalVariables|GetAdded%20Text%20Render%20Comp) _array_element)))))
      (:then_1
        ;[1 1 1] Root Offset
        (Transformation|AddRelativeLocation Parent Offset false false)))))