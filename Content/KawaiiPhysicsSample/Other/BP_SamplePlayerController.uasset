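; Player controller for the KawaiiPhysics sample maps, showing an on-screen key guide and toggling debug draw, slow motion and a simulation space setting.
; Exhibit and category jumps parse "N.M" numbers on BP_KPS_ExhibitPlate actors, cycle with wraparound and teleport the pawn to a framed view.
; Docs and AnimBP shortcuts open the last-jumped plate while the camera stays there, otherwise the nearest eligible plate.
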(event Input|EnhancedActionEvents|EnhancedInputActionIA_ChangeSimSpace
  (params (ActionValue :type Boolean) (ElapsedSeconds :type Float%20%28double-precision%29) (TriggeredSeconds :type Float%20%28double-precision%29) (InputAction :type Input%20Action%20Object%20Reference :default "/Game/KawaiiPhysicsSample/Other/Input/IA_ChangeSimSpace.IA_ChangeSimSpace"))
  ;[1 1 1] Input
  (bind _isa (Utilities|FlowControl|FlipFlop)
    (:A
      _)
    (:B
      _))
  (Variables|Default|SetSimulationSpace (select _isa "WorldSpace" "ComponentSpace")))

(event Input|EnhancedActionEvents|EnhancedInputActionIA_ToggleDebug
  (params (ActionValue :type Boolean) (ElapsedSeconds :type Float%20%28double-precision%29) (TriggeredSeconds :type Float%20%28double-precision%29) (InputAction :type Input%20Action%20Object%20Reference :default "/Game/KawaiiPhysicsSample/Other/Input/IA_ToggleDebug.IA_ToggleDebug"))
  ;[1 1 1] Input
  (bind _returnvalue (Development|GetConsoleVariableBoolValue "a.AnimNode.KawaiiPhysics.Debug"))
  (Development|ExecuteConsoleCommand (Utilities|String|Append "a.AnimNode.KawaiiPhysics.Debug " (Utilities|String|ToString(Boolean) (not _returnvalue))) 0))

(event Input|EnhancedActionEvents|EnhancedInputActionIA_PrevExhibit
  (params (ActionValue :type Boolean) (ElapsedSeconds :type Float%20%28double-precision%29) (TriggeredSeconds :type Float%20%28double-precision%29) (InputAction :type Input%20Action%20Object%20Reference :default "/Game/KawaiiPhysicsSample/Other/Input/IA_PrevExhibit.IA_PrevExhibit"))
  ;[0.15 0.15 0.15 0.5] Debug exhibit jump (L_KPS_AllExamples): Z / X = previous / next exhibit, PageUp / PageDown = previous / next category
  (CallFunction|JumpExhibit -1))

(event Input|EnhancedActionEvents|EnhancedInputActionIA_ToggleSlomo
  (params (ActionValue :type Boolean) (ElapsedSeconds :type Float%20%28double-precision%29) (TriggeredSeconds :type Float%20%28double-precision%29) (InputAction :type Input%20Action%20Object%20Reference :default "/Game/KawaiiPhysicsSample/Other/Input/IA_ToggleSlomo.IA_ToggleSlomo"))
  ;[1 1 1] Input
  (Utilities|Time|SetGlobalTimeDilation (Math|Float|SelectFloat 0.2 1.0 (Math|Float|NearlyEqual(Float) (Class|GameplayStatics|GetGlobalTimeDilation) 1.0 1e-06))))

(event Input|EnhancedActionEvents|EnhancedInputActionIA_NextExhibit
  (params (ActionValue :type Boolean) (ElapsedSeconds :type Float%20%28double-precision%29) (TriggeredSeconds :type Float%20%28double-precision%29) (InputAction :type Input%20Action%20Object%20Reference :default "/Game/KawaiiPhysicsSample/Other/Input/IA_NextExhibit.IA_NextExhibit"))
  ;[0.15 0.15 0.15 0.5] Debug exhibit jump (L_KPS_AllExamples): Z / X = previous / next exhibit, PageUp / PageDown = previous / next category
  (CallFunction|JumpExhibit 1))

(event Input|EnhancedActionEvents|EnhancedInputActionIA_PrevCategory
  (params (ActionValue :type Boolean) (ElapsedSeconds :type Float%20%28double-precision%29) (TriggeredSeconds :type Float%20%28double-precision%29) (InputAction :type Input%20Action%20Object%20Reference :default "/Game/KawaiiPhysicsSample/Other/Input/IA_PrevCategory.IA_PrevCategory"))
  ;[0.15 0.15 0.15 0.5] Debug exhibit jump (L_KPS_AllExamples): Z / X = previous / next exhibit, PageUp / PageDown = previous / next category
  (CallFunction|JumpCategory -1))

(event Input|EnhancedActionEvents|EnhancedInputActionIA_NextCategory
  (params (ActionValue :type Boolean) (ElapsedSeconds :type Float%20%28double-precision%29) (TriggeredSeconds :type Float%20%28double-precision%29) (InputAction :type Input%20Action%20Object%20Reference :default "/Game/KawaiiPhysicsSample/Other/Input/IA_NextCategory.IA_NextCategory"))
  ;[0.15 0.15 0.15 0.5] Debug exhibit jump (L_KPS_AllExamples): Z / X = previous / next exhibit, PageUp / PageDown = previous / next category
  (CallFunction|JumpCategory 1))

(event Input|EnhancedActionEvents|EnhancedInputActionIA_OpenDocs
  (params (ActionValue :type Boolean) (ElapsedSeconds :type Float%20%28double-precision%29) (TriggeredSeconds :type Float%20%28double-precision%29) (InputAction :type Input%20Action%20Object%20Reference :default "/Game/KawaiiPhysicsSample/Other/Input/IA_OpenDocs.IA_OpenDocs"))
  (bind _plate (CallFunction|FindDocsPlate false))
  (if (Utilities|IsValid _plate)
    (Development|PrintString (Utilities|String|Append "Open Docs: " (Default|GetDocURL _plate)) true true "(R=0.000000,G=0.660000,B=1.000000,A=1.000000)" 3.0 "OpenDocs")
    (Default|OpenDocs _plate)
    (else
      (Development|PrintString "No docs page for the nearby exhibit" true true "(R=0.000000,G=0.660000,B=1.000000,A=1.000000)" 3.0 "OpenDocs"))))

(event Input|EnhancedActionEvents|EnhancedInputActionIA_OpenAnimBP
  (params (ActionValue :type Boolean) (ElapsedSeconds :type Float%20%28double-precision%29) (TriggeredSeconds :type Float%20%28double-precision%29) (InputAction :type Input%20Action%20Object%20Reference :default "/Game/KawaiiPhysicsSample/Other/Input/IA_OpenAnimBP.IA_OpenAnimBP"))
  (bind _plate (CallFunction|FindDocsPlate true))
  (if (Utilities|IsValid _plate)
    (Development|PrintString (Utilities|String|Append "Open AnimBP: " (Default|GetAnimBlueprintPath _plate)) true true "(R=0.000000,G=0.660000,B=1.000000,A=1.000000)" 3.0 "OpenAnimBP")
    (Default|OpenAnimBlueprint _plate)
    (else
      (Development|PrintString "No AnimBP for the nearby exhibit" true true "(R=0.000000,G=0.660000,B=1.000000,A=1.000000)" 3.0 "OpenAnimBP"))))

(event EventBeginPlay
  (bind _returnvalue (Game|GetPlayerController 0))
  ;[1 1 1] BeginPlay
  (Variables|/Script/Engine.PlayerCameraManager|SetDefaultFOV (Game|GetPlayerCameraManager 0) 45.0)
  (Input|EnableInput _returnvalue)
  (Input|AddMappingContext (PlayerController|LocalPlayerSubsystems|GetEnhancedInputLocalPlayerSubsystem _returnvalue) "/Game/KawaiiPhysicsSample/Other/Input/IMC_Sample.IMC_Sample" 0 "(bIgnoreAllPressedKeysUntilRelease=True,bForceImmediately=False,bNotifyUserSettings=False)"))

(event EventTick
  (params (DeltaSeconds :type Float%20%28single-precision%29))
  ;[1 1 1] Tick
  (|CallParentFunction DeltaSeconds)
  (Development|PrintText (Utilities|Text|FormatText "1: Toggle Show Debug 
2: Toggle Slomo 
3: Change Sim Space ({Space}) 
Z / X: Prev / Next Exhibit 
PgUp / PgDn: Prev / Next Category" (Utilities|String|EnumtoString (Variables|Default|GetSimulationSpace))) true false "(R=1.000000,G=1.000000,B=1.000000,A=1.000000)" 0.0))

(fn ConstructionScript)

(fn GetCurrentStageIndex
  (return (Math|Float|Floor (/ (.y (Transformation|GetActorLocation (Game|Player|GetPlayerPawn 0))) 1e+03))))

(fn ParsePlateNumber
  (params (Number :type String))
  (bind (_lefts _rights) (Utilities|String|Split Number "."))
  ;[0.15 0.15 0.15 0.5] Parse an exhibit plate Number: "N.M" -> Category N, Exhibit M; intro / overview "NN" -> Category NN, Exhibit 0
  (if (Utilities|String|Contains Number ".")
    (return (Math|Conversions|ToInteger(Byte) _lefts) (Math|Conversions|ToInteger(Byte) _rights))
    (else
      (return (Math|Conversions|ToInteger(Byte) Number) 0))))

(fn MovetoPlate
  (params (Plate :type BP%20KPS%20Exhibit%20Plate%20Object%20Reference))
  (bind _returnvalue (Transformation|GetActorLocation Plate))
  (bind _returnvalue_2 (Transformation|GetActorForwardVector Plate))
  (bind _self self)
  (bind _number (Variables|/Game/KawaiiPhysicsSample/Examples/Common/BP_KPS_ExhibitPlate.BP_KPS_ExhibitPlate_C|GetNumber Plate))
  (bind _jumpviewdistance (Variables|ExhibitJump|GetJumpViewDistance))
  (bind _jumpviewheight (Variables|ExhibitJump|GetJumpViewHeight))
  (bind _returnvalue_3 (Pawn|GetControlledPawn _self))
  (bind _returnvalue_4 (Math|Vector|MakeVector 0.0 0.0 _jumpviewheight))
  (bind _returnvalue_5 (Utilities|String|ToString(Text) _number))
  (bind _returnvalue_6 (* _returnvalue_2 _jumpviewdistance))
  (bind _returnvalue_7 (- _returnvalue _returnvalue_6))
  (bind _returnvalue_8 (+ _returnvalue_7 _returnvalue_4))
  ;[0.15 0.15 0.15 0.5] Put the pawn JumpViewDistance in front of the plate and JumpViewHeight above its base, look at it with JumpViewPitch (framed so the board top and the deck front edge fit a 2:1 or 16:9 view at the 45 deg FOV set in BeginPlay), store it as the current exhibit and show its number and title
  ;;[0.15 0.15 0.15 0.5] Put the pawn 900 cm in front of the plate and 170 cm above it, face the plate, store it as the current exhibit and show its number and title
  (Utilities|IsValid _returnvalue_3
    (:Is%20Valid
      (Variables|Default|SetJumpCameraLocation (+ _returnvalue_8 (- (Camera|GetCameraLocation (Game|GetPlayerCameraManager 0)) (Transformation|GetActorLocation _returnvalue_3))))
      (Variables|Default|SetbHasJumped true)
      (Transformation|SetActorLocation _returnvalue_3 _returnvalue_8 false true)
      (Pawn|SetControlRotation _self (Math|Rotator|MakeRotator 0.0 (Variables|ExhibitJump|GetJumpViewPitch) (.Yaw (Math|Rotator|BreakRotator (Transformation|GetActorRotation Plate)))))
      (bind (_category _exhibit) (CallFunction|ParsePlateNumber _returnvalue_5))
      (Variables|ExhibitJump|SetCurrentCategory _category)
      (Variables|ExhibitJump|SetCurrentExhibit _exhibit)
      (Development|PrintString (Utilities|String|Append (Utilities|String|Append _returnvalue_5 "  ") (Utilities|String|ToString(Text) (Variables|/Game/KawaiiPhysicsSample/Examples/Common/BP_KPS_ExhibitPlate.BP_KPS_ExhibitPlate_C|GetTitle Plate))) true true "(R=0.000000,G=0.660000,B=1.000000,A=1.000000)" 3.0 "ExhibitJump"))))

(fn EnsureCurrentPlate
  (bind _self self)
  (bind _returnvalue (Pawn|GetControlledPawn _self))
  ;[0.15 0.15 0.15 0.5] If no loaded plate matches CurrentCategory / CurrentExhibit (first press, or its level is not loaded), adopt the plate nearest to the pawn
  (bind _outactors (Actor|GetAllActorsOfClass "/Game/KawaiiPhysicsSample/Examples/Common/BP_KPS_ExhibitPlate.BP_KPS_ExhibitPlate_C"))
  (for _array_element _outactors
    (bind (_category _exhibit) (CallFunction|ParsePlateNumber (Utilities|String|ToString(Text) (Variables|/Game/KawaiiPhysicsSample/Examples/Common/BP_KPS_ExhibitPlate.BP_KPS_ExhibitPlate_C|GetNumber _array_element))))
    (if (and (== _category (Variables|ExhibitJump|GetCurrentCategory)) (== _exhibit (Variables|ExhibitJump|GetCurrentExhibit)))
      (LocalVariables|SetbFound true)))
  (if (not (LocalVariables|GetbFound))
    (Utilities|IsValid _returnvalue
      (:Is%20Valid
        (LocalVariables|SetNearestDistance 1e+08)
        (for _array_element_2 _outactors
          (if (< (Math|Vector|Distance(Vector) (Transformation|GetActorLocation _array_element_2) (Transformation|GetActorLocation _returnvalue)) (LocalVariables|GetNearestDistance))
            (LocalVariables|SetNearestDistance (Math|Vector|Distance(Vector) (Transformation|GetActorLocation _array_element_2) (Transformation|GetActorLocation _returnvalue)))
            (LocalVariables|SetNearestPlate _array_element_2)))
        (Utilities|IsValid (LocalVariables|GetNearestPlate)
          (:Is%20Valid
            (bind (_category_2 _exhibit_2) (CallFunction|ParsePlateNumber (Utilities|String|ToString(Text) (Variables|/Game/KawaiiPhysicsSample/Examples/Common/BP_KPS_ExhibitPlate.BP_KPS_ExhibitPlate_C|GetNumber (LocalVariables|GetNearestPlate)))))
            (Variables|ExhibitJump|SetCurrentCategory _category_2)
            (Variables|ExhibitJump|SetCurrentExhibit _exhibit_2)))))))

(fn JumpExhibit
  (params (Direction :type Integer))
  ;[0.15 0.15 0.15 0.5] Within CurrentCategory pick the next exhibit in Direction (key = Exhibit * Direction, smallest key above the current one); wrap to the smallest key. Nothing happens when no plates exist
  (CallFunction|EnsureCurrentPlate)
  (LocalVariables|SetBestKey 2147483647)
  (LocalVariables|SetWrapKey 2147483647)
  (bind _outactors (Actor|GetAllActorsOfClass "/Game/KawaiiPhysicsSample/Examples/Common/BP_KPS_ExhibitPlate.BP_KPS_ExhibitPlate_C"))
  (for _array_element _outactors
    (bind (_category _exhibit) (CallFunction|ParsePlateNumber (Utilities|String|ToString(Text) (Variables|/Game/KawaiiPhysicsSample/Examples/Common/BP_KPS_ExhibitPlate.BP_KPS_ExhibitPlate_C|GetNumber _array_element))))
    (if (== _category (Variables|ExhibitJump|GetCurrentCategory))
      (if (and (> (* _exhibit Direction) (* (Variables|ExhibitJump|GetCurrentExhibit) Direction)) (< (* _exhibit Direction) (LocalVariables|GetBestKey)))
        (LocalVariables|SetBestKey (* _exhibit Direction))
        (LocalVariables|SetBestPlate _array_element))
      (if (< (* _exhibit Direction) (LocalVariables|GetWrapKey))
        (LocalVariables|SetWrapKey (* _exhibit Direction))
        (LocalVariables|SetWrapPlate _array_element))))
  (if (< (LocalVariables|GetBestKey) (Class|KismetSystemLibrary|MakeLiteralInteger 2147483647))
    (CallFunction|MovetoPlate (LocalVariables|GetBestPlate))
    (else
      (Utilities|IsValid (LocalVariables|GetWrapPlate)
        (:Is%20Valid
          (CallFunction|MovetoPlate (LocalVariables|GetWrapPlate)))))))

(fn JumpCategory
  (params (Direction :type Integer))
  ;[0.15 0.15 0.15 0.5] Pick the next existing category in Direction (key = Category * Direction), wrapping around (0 = overview is part of the cycle), then land on its lowest exhibit (intro / overview)
  (CallFunction|EnsureCurrentPlate)
  (LocalVariables|SetBestKey 2147483647)
  (LocalVariables|SetWrapKey 2147483647)
  (LocalVariables|SetLowestExhibit 2147483647)
  (bind _outactors (Actor|GetAllActorsOfClass "/Game/KawaiiPhysicsSample/Examples/Common/BP_KPS_ExhibitPlate.BP_KPS_ExhibitPlate_C"))
  (for _array_element _outactors
    (bind _category (CallFunction|ParsePlateNumber (Utilities|String|ToString(Text) (Variables|/Game/KawaiiPhysicsSample/Examples/Common/BP_KPS_ExhibitPlate.BP_KPS_ExhibitPlate_C|GetNumber _array_element))))
    (if (and (> (* _category Direction) (* (Variables|ExhibitJump|GetCurrentCategory) Direction)) (< (* _category Direction) (LocalVariables|GetBestKey)))
      (LocalVariables|SetBestKey (* _category Direction)))
    (if (< (* _category Direction) (LocalVariables|GetWrapKey))
      (LocalVariables|SetWrapKey (* _category Direction))))
  (if (< (LocalVariables|GetBestKey) (Class|KismetSystemLibrary|MakeLiteralInteger 2147483647))
    (LocalVariables|SetTargetCategory (* (LocalVariables|GetBestKey) Direction))
    (else
      (LocalVariables|SetTargetCategory (* (LocalVariables|GetWrapKey) Direction))))
  (for _array_element_2 _outactors
    (bind (_category_2 _exhibit) (CallFunction|ParsePlateNumber (Utilities|String|ToString(Text) (Variables|/Game/KawaiiPhysicsSample/Examples/Common/BP_KPS_ExhibitPlate.BP_KPS_ExhibitPlate_C|GetNumber _array_element_2))))
    (if (and (== _category_2 (LocalVariables|GetTargetCategory)) (< _exhibit (LocalVariables|GetLowestExhibit)))
      (LocalVariables|SetLowestExhibit _exhibit)
      (LocalVariables|SetTargetPlate _array_element_2)))
  (Utilities|IsValid (LocalVariables|GetTargetPlate)
    (:Is%20Valid
      (CallFunction|MovetoPlate (LocalVariables|GetTargetPlate)))))

(fn FindDocsPlate
  (params (bRequireAnimBP :type Boolean))
  (LocalVariables|SetViewLoc (Camera|GetCameraLocation (Game|GetPlayerCameraManager 0)))
  (bind _outactors (Actor|GetAllActorsOfClass "/Game/KawaiiPhysicsSample/Examples/Common/BP_KPS_ExhibitPlate.BP_KPS_ExhibitPlate_C"))
  (for _array_element _outactors
    (if (not (or (Utilities|Array|IsEmpty (Variables|/Game/KawaiiPhysicsSample/Examples/Common/BP_KPS_ExhibitPlate.BP_KPS_ExhibitPlate_C|GetDocPath _array_element)) (and bRequireAnimBP (not (Utilities|IsValidSoftClassReference (Variables|/Game/KawaiiPhysicsSample/Examples/Common/BP_KPS_ExhibitPlate.BP_KPS_ExhibitPlate_C|GetAnimBlueprint _array_element))))))
      (if (< (Math|Vector|Distance(Vector) (Transformation|GetActorLocation _array_element) (LocalVariables|GetViewLoc)) (LocalVariables|GetBestDist))
        (LocalVariables|SetBestDist (Math|Vector|Distance(Vector) (Transformation|GetActorLocation _array_element) (LocalVariables|GetViewLoc)))
        (LocalVariables|SetBestPlate _array_element))
      (bind (_category _exhibit) (CallFunction|ParsePlateNumber (Utilities|String|ToString(Text) (Variables|/Game/KawaiiPhysicsSample/Examples/Common/BP_KPS_ExhibitPlate.BP_KPS_ExhibitPlate_C|GetNumber _array_element))))
      (if (and (== _category (Variables|ExhibitJump|GetCurrentCategory)) (== _exhibit (Variables|ExhibitJump|GetCurrentExhibit)))
        (LocalVariables|SetCurDist (Math|Vector|Distance(Vector) (Transformation|GetActorLocation _array_element) (LocalVariables|GetViewLoc)))
        (LocalVariables|SetCurPlate _array_element))))
  (if (and (Utilities|IsValid (LocalVariables|GetCurPlate)) (and (Variables|Default|GetbHasJumped) (<= (Math|Vector|Distance(Vector) (LocalVariables|GetViewLoc) (Variables|Default|GetJumpCameraLocation)) 1e+02)))
    (return (LocalVariables|GetCurPlate))
    (else
      (return (LocalVariables|GetBestPlate)))))